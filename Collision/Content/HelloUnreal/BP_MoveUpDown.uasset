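; Actor that bounces a Cube component vertically between local Z zero and EndPoint while IsPlay is true.
; Tick moves it a fixed step per frame, independent of delta time, and flips IsMoveUp at each limit.
; BeginPlay binds an event to the ThirdPersonCharacter's F-key dispatcher, with an auto-generated handler that sets IsPlay from the pressed state.
; Play and Stop functions also set IsPlay from their input.
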(event `self.ReceiveTick`
  (params (DeltaSeconds :type "Float (single-precision)"))
  (bind _cube (`self.Cube`))
  (bind (_relativelocation_x _relativelocation_y _relativelocation_z) (`KismetMathLibrary.BreakVector` (`SceneComponent.RelativeLocation` _cube)))
  (bind (_relativelocation_x_2 _relativelocation_y_2 _relativelocation_z_2) (`KismetMathLibrary.BreakVector` (`SceneComponent.RelativeLocation` _cube)))
  (if (`self.IsPlay`)
    (if (`self.IsMoveUp`)
      (`SceneComponent.K2_AddRelativeLocation` _cube (0.0 0.0 5.0) false false)
      (if (>= _relativelocation_z_2 (`self.EndPoint`))
        (set `self.IsMoveUp` false))
      (else
        (`SceneComponent.K2_AddRelativeLocation` (`self.Cube`) (0.0 0.0 -5.0) false false)
        (if (< _relativelocation_z 0.0)
          (set `self.IsMoveUp` true))))))

(event `self.ReceiveBeginPlay`
  (bind _asthird_person_character (cast `/Game/ThirdPersonBP/Blueprints/ThirdPersonCharacter` (`GameplayStatics.GetPlayerCharacter` 0)))
  (add `/Game/ThirdPersonBP/Blueprints/ThirdPersonCharacter.EventDispatcher_F_key` _asthird_person_character (`|CreateDelegate` :!event `BP_MoveUpDown_AutoGenFunc`)))

(fn `BP_MoveUpDown_AutoGenFunc`
  (params (isPressed :type Boolean))
  (set `self.IsPlay` isPressed))

(fn `Play`
  (params (IsPlay :type Boolean))
  (returns (Result :type Boolean))
  (set `self.IsPlay` IsPlay)
  (return false))

(fn `Stop`
  (params (`Is Play` :type Boolean))
  (returns (Result :type Boolean))
  (set `self.IsPlay` `Is Play`)
  (return false))

(fn `UserConstructionScript`)