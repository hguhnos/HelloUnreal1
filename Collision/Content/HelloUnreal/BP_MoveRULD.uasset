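; BP_MoveRULD is an actor that moves its Cube around a square path in the X-Z plane: right, up, left, then down, repeating.
; While IsPlay is set, Tick switches on a direction enum, applies a fixed per-frame relative offset without sweep, and advances direction at EndPoint or zero.
; BeginPlay binds to the ThirdPersonCharacter's F-key dispatcher, with a generated handler that copies IsPressed into IsPlay.
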(event `self.ReceiveTick`
  (params (DeltaSeconds :type "Float (single-precision)"))
  (bind _cube (`self.Cube`))
  (bind _cube_2 (`self.Cube`))
  (bind _cube_3 (`self.Cube`))
  (bind _cube_4 (`self.Cube`))
  (bind (_relativelocation_x _relativelocation_y _relativelocation_z) (`KismetMathLibrary.BreakVector` (`SceneComponent.RelativeLocation` _cube_4)))
  (bind _relativelocation_x_2 (`KismetMathLibrary.BreakVector` (`SceneComponent.RelativeLocation` _cube)))
  (bind (_relativelocation_x_3 _relativelocation_y_2 _relativelocation_z_2) (`KismetMathLibrary.BreakVector` (`SceneComponent.RelativeLocation` _cube_2)))
  (bind _relativelocation_x_4 (`KismetMathLibrary.BreakVector` (`SceneComponent.RelativeLocation` _cube_3)))
  (if (`self.IsPlay`)
    (switch `/Game/HelloUnreal/EN_MoveType` (`self.En_MoveTyPE`)
      (:`NewEnumerator0`
        ;[1 1 1] 오른쪽으로 이동
        (`SceneComponent.K2_AddRelativeLocation` _cube_3 (5.0 0.0 0.0) false false)
        (if (>= _relativelocation_x_4 (`self.EndPoint`))
          (set `self.En_MoveTyPE` "NewEnumerator1")))
      (:`NewEnumerator1`
        ;[1 1 1] 위쪽으로 이동
        (`SceneComponent.K2_AddRelativeLocation` _cube_4 (0.0 0.0 5.0) false false)
        (if (>= _relativelocation_z (`self.EndPoint`))
          (set `self.En_MoveTyPE` "NewEnumerator2")))
      (:`NewEnumerator2`
        ;[1 1 1] 왼쪽으로 이동
        (`SceneComponent.K2_AddRelativeLocation` _cube (-5.0 0.0 0.0) false false)
        (if (>= 0.0 _relativelocation_x_2)
          (set `self.En_MoveTyPE` "NewEnumerator3")))
      (:`NewEnumerator3`
        ;[1 1 1] 아래쪽으로 이동
        (`SceneComponent.K2_AddRelativeLocation` _cube_2 (0.0 0.0 -5.0) false false)
        (if (>= 0.0 _relativelocation_z_2)
          (set `self.En_MoveTyPE` "NewEnumerator0"))))))

(event `self.ReceiveBeginPlay`
  (bind _asthird_person_character (cast `/Game/ThirdPersonBP/Blueprints/ThirdPersonCharacter` (`GameplayStatics.GetPlayerCharacter` 0)))
  (add `/Game/ThirdPersonBP/Blueprints/ThirdPersonCharacter.EventDispatcher_F_key` _asthird_person_character (`|CreateDelegate` :!event `BP_MoveRULD_AutoGenFunc`)))

(fn `BP_MoveRULD_AutoGenFunc`
  (params (isPressed :type Boolean))
  (set `self.IsPlay` isPressed))

(fn `Play`
  (params (IsPlay :type Boolean))
  (returns (Result :type Boolean))
  (set `self.IsPlay` IsPlay)
  (return true))

(fn `Stop`
  (params (`Is Play` :type Boolean))
  (returns (Result :type Boolean))
  (set `self.IsPlay` false)
  (return false))

(fn `UserConstructionScript`)