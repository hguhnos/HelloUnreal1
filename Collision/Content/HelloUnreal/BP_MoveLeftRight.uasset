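; BP_MoveLeftRight is an actor whose Cube slides back and forth along its relative X axis while play is enabled.
; Tick moves it by a fixed per-frame offset, unscaled by delta time, reversing at EndPoint and below zero.
; BeginPlay binds to the ThirdPersonCharacter's F-key event dispatcher, whose pressed state drives IsPlay.
; A separate Play function also sets that flag.
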(event `self.ReceiveTick`
  (params (DeltaSeconds :type "Float (single-precision)"))
  (bind _cube (`self.Cube`))
  (bind _relativelocation_x (`KismetMathLibrary.BreakVector` (`SceneComponent.RelativeLocation` _cube)))
  (bind _relativelocation_x_2 (`KismetMathLibrary.BreakVector` (`SceneComponent.RelativeLocation` _cube)))
  (if (`self.IsPlay`)
    (if (`self.IsMoveRight`)
      (`SceneComponent.K2_AddRelativeLocation` _cube (5.0 0.0 0.0) false false)
      (if (>= _relativelocation_x_2 (`self.EndPoint`))
        (set `self.IsMoveRight` false))
      (else
        (`SceneComponent.K2_AddRelativeLocation` (`self.Cube`) (-5.0 0.0 0.0) false false)
        (if (< _relativelocation_x 0.0)
          (set `self.IsMoveRight` true))))))

(event `self.ReceiveBeginPlay`
  (bind _asthird_person_character (cast `/Game/ThirdPersonBP/Blueprints/ThirdPersonCharacter` (`GameplayStatics.GetPlayerCharacter` 0)))
  (add `/Game/ThirdPersonBP/Blueprints/ThirdPersonCharacter.EventDispatcher_F_key` _asthird_person_character (`|CreateDelegate` :!event `BindEvent_F_key`)))

(fn `BindEvent_F_key`
  (params (isPressed :type Boolean))
  (set `self.IsPlay` isPressed))

(fn `Play`
  (params (IsPlay :type Boolean))
  (returns (Result :type Boolean))
  (set `self.IsPlay` IsPlay)
  (return true))

(fn `UserConstructionScript`)