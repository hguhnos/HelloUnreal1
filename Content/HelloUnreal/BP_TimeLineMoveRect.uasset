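; Actor Blueprint that moves its Sphere component endlessly around a rectangular path in the relative XZ plane, starting on BeginPlay.
; A Movetype state selects whether one shared timeline plays forward (Right, Up) or in reverse (Left, Down).
; UpdateMove scales the timeline value by EndPoint and applies it to X or Z.
; On finish, ChangeMoveType advances Right, Up, Left, Down and re-enters the state switch.
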(event `self.ReceiveBeginPlay`
  ;[1 1 1] 상태에 따른 실행라인 방향처리
  (switch `/Game/HelloUnreal/EN_MoveType` (`self.Movetype`) :!label _label
    (:`NewEnumerator0`
      (bind (_direction _value) (`Timeline|타임라인_0` :!via `PlayFromStart` :!label _label_2)
        (:`Update`
          (`self.Update Move` _value))
        (:`Finished`
          (`self.Change Move Type`)
          (goto _label))))
    (:`NewEnumerator1`
      (goto _label_2 :!via `PlayFromStart`))
    (:`NewEnumerator2`
      (goto _label_2 :!via `ReverseFromEnd`))
    (:`NewEnumerator3`
      (goto _label_2 :!via `ReverseFromEnd`))))

(fn `Change Move Type`
  ;[1 1 1] 방향 바꾸기
  (switch `/Game/HelloUnreal/EN_MoveType` (`self.Movetype`)
    (:`NewEnumerator0`
      (set `self.Movetype` "NewEnumerator1"))
    (:`NewEnumerator1`
      (set `self.Movetype` "NewEnumerator2"))
    (:`NewEnumerator2`
      (set `self.Movetype` "NewEnumerator3"))
    (:`NewEnumerator3`
      (set `self.Movetype` "NewEnumerator0"))))

(fn `Update Move`
  (params (Value :type "Float (double-precision)"))
  (bind _sphere (`self.Sphere`))
  (bind _sphere_2 (`self.Sphere`))
  (bind _returnvalue (* Value (`self.EndPoint`)))
  (bind (_relativelocation_x _relativelocation_y _relativelocation_z) (`KismetMathLibrary.BreakVector` (`SceneComponent.RelativeLocation` _sphere_2)))
  (bind (_relativelocation_x_2 _relativelocation_y_2) (`KismetMathLibrary.BreakVector` (`SceneComponent.RelativeLocation` _sphere)))
  (switch `/Game/HelloUnreal/EN_MoveType` (`self.Movetype`)
    (:`NewEnumerator0`
      (`SceneComponent.K2_SetRelativeLocation` _sphere_2 (`KismetMathLibrary.MakeVector` _returnvalue _relativelocation_y _relativelocation_z) false false :!label _label))
    (:`NewEnumerator1`
      (`SceneComponent.K2_SetRelativeLocation` _sphere (`KismetMathLibrary.MakeVector` _relativelocation_x_2 _relativelocation_y_2 _returnvalue) false false :!label _label_2))
    (:`NewEnumerator2`
      (goto _label))
    (:`NewEnumerator3`
      (goto _label_2))))

(fn `UserConstructionScript`)